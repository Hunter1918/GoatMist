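; Pushable cannon that the first-person player can take control of, move around and fire.
; The interaction box registers the cannon on the overlapping character and toggles a prompt that turns to face the camera each Tick.
; While controlled, Tick passes move input to the player and sweeps the cannon in front of the camera, keeping its height and matching camera yaw.
; Firing spawns a cannonball at FirePoint, gated by a short cooldown.
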(event OnComponentBeginOverlap(BoxCollision_Interaction)
  (params (OverlappedComponent :type Primitive%20Component%20Object%20Reference) (OtherActor :type Actor%20Object%20Reference) (OtherComp :type Primitive%20Component%20Object%20Reference) (OtherBodyIndex :type Integer) (bFromSweep :type Boolean) (SweepResult :type Hit%20Result%20Structure%20%28by%20ref%29))
  (bind _asbp_first_person_character (Utilities|Casting|CastToBP_FirstPersonCharacter OtherActor))
  (Variables|/Game/Ugu/FirstPerson/Blueprints/BP_FirstPersonCharacter.BP_FirstPersonCharacter_C|SetInteractableCanon _asbp_first_person_character self)
  (Variables|Default|SetPlayerRef _asbp_first_person_character)
  (Variables|Default|SetbCanInteract true)
  (Development|PrintString "Utiliser Le Canon appuie sur E la ptn de ta race nan mais SERIEUX mais que fait mon teamate (coup d'accoudoir)")
  (Rendering|SetVisibility (Variables|Default|GetInteract) true false))

(event OnComponentEndOverlap(BoxCollision_Interaction)
  (params (OverlappedComponent :type Primitive%20Component%20Object%20Reference) (OtherActor :type Actor%20Object%20Reference) (OtherComp :type Primitive%20Component%20Object%20Reference) (OtherBodyIndex :type Integer))
  (bind _asbp_first_person_character (Utilities|Casting|CastToBP_FirstPersonCharacter OtherActor))
  (Variables|/Game/Ugu/FirstPerson/Blueprints/BP_FirstPersonCharacter.BP_FirstPersonCharacter_C|SetInteractableCanon _asbp_first_person_character 0)
  (Variables|Default|SetPlayerRef _asbp_first_person_character)
  (Variables|Default|SetbCanInteract false)
  (Development|PrintString "Cache moi le texte mais SERIEUX INVITE PK IL INVITE JAMAIIIIIIIIIIIIIIIIIS")
  (Rendering|SetVisibility (Variables|Default|GetInteract) false false))

(event Custom|SetMoveInput
  (params (Input :type Vector%202D%20Structure))
  (bind _output_get (Variables|Default|SetMoveInput Input)))

(event Custom|PushCanon
  (bind _returnvalue (Game|GetPlayerCameraManager 0))
  (bind _playerref (Variables|Default|GetPlayerRef))
  (bind _returnvalue_2 (Camera|GetCameraLocation _returnvalue))
  (bind _returnvalue_3 (Camera|GetCameraRotation _returnvalue))
  (bind _returnvalue_4 (Math|Vector|GetForwardVector _returnvalue_3))
  (bind _returnvalue_5 (* _returnvalue_2 1.0))
  (bind _returnvalue_6 (* _returnvalue_4 1.5e+02))
  (bind _returnvalue_7 (+ _returnvalue_6 _returnvalue_5))
  (if (Variables|Default|GetbIsControlled)
    (Utilities|IsValid _playerref
      (:Is%20Valid
        (Variables|/Game/Ugu/FirstPerson/Blueprints/BP_FirstPersonCharacter.BP_FirstPersonCharacter_C|SetMoveInput _playerref (stale Custom|SetMoveInput _output_get))
        (Transformation|SetActorLocation (Math|Vector|MakeVector (.x _returnvalue_7) (.y _returnvalue_7) (.z (Transformation|GetActorLocation))) true false)
        (Transformation|SetActorRotation (Math|Rotator|MakeRotator 0.0 0.0 (.yaw (Camera|GetCameraRotation (Game|GetPlayerCameraManager 0)))))))))

(event Custom|FireCannon
  (if (Variables|Default|GetCanFire)
    (Variables|Default|SetCanFire false)
    (Game|SpawnActorfromClass (Variables|Default|GetCannonBallClass) (Transformation|GetWorldTransform (Variables|Default|GetFirePoint)) "Undefined" "MultiplyWithRoot" 0 0)
    (Utilities|FlowControl|Delay 2.0)
    (Variables|Default|SetCanFire true)))

(event Custom|StartControl
  (Variables|Default|SetbIsControlled true)
  (Rendering|SetVisibility (Variables|Default|GetInteract) false false))

(event Custom|StopControl
  (Variables|Default|SetbIsControlled false)
  (Rendering|SetVisibility (Variables|Default|GetInteract) true false))

(event EventTick
  (params (DeltaSeconds :type Float%20%28single-precision%29))
  (Variables|Default|SetDelta%20Seconds DeltaSeconds)
  (CallFunction|PushCanon)
  (Transformation|SetWorldRotation (Variables|Default|GetInteract) (Math|Rotator|FindLookatRotation (Transformation|GetWorldLocation (Variables|Default|GetInteract)) (Camera|GetCameraLocation (Game|GetPlayerCameraManager 0))) false false))

(event EventBeginPlay
  (Rendering|SetVisibility (Variables|Default|GetInteract) false false))

(fn ConstructionScript)