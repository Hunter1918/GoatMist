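; Breakable plank that a cannonball destroys during a two-second window opened by CanBreak, triggering a scripted cutscene.
; The hit decrements the player's cannonball count, drops linked crates and plank, and destroys the actor stored by CanBreak.
; The sequence moves and reorients the player, enables hold-door opening, then branches on EntrePont to the prison widget and QTE actors or a falling plank.
; Remove_UI clears that widget and plays a hint sequence before restoring input.
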(event OnComponentBeginOverlap(Box)
  (params (OverlappedComponent :type Primitive%20Component%20Object%20Reference) (OtherActor :type Actor%20Object%20Reference) (OtherComp :type Primitive%20Component%20Object%20Reference) (OtherBodyIndex :type Integer) (bFromSweep :type Boolean) (SweepResult :type Hit%20Result%20Structure%20%28by%20ref%29))
  (Utilities|Casting|CastToBP_Boulet_De_Canon OtherActor)
  (bind _asbp_first_person_character (Utilities|Casting|CastToBP_FirstPersonCharacter (Game|GetPlayerCharacter 0)))
  (Variables|Default|SetAs%20BP%20First%20Person%20Character _asbp_first_person_character)
  (Variables|/Game/Ugu/FirstPerson/Blueprints/BP_FirstPersonCharacter.BP_FirstPersonCharacter_C|SetNbrOfBoulet _asbp_first_person_character (- (Variables|/Game/Ugu/FirstPerson/Blueprints/BP_FirstPersonCharacter.BP_FirstPersonCharacter_C|GetNbrOfBoulet _asbp_first_person_character) 1))
  (Variables|/Script/Engine.PrimitiveComponent|SetbGenerateOverlapEvents (Variables|Default|GetBox) false)
  (Default|Drop (Variables|Default|GetREF_Caisse))
  (Default|Drop (Variables|Default|GetREF_Planche))
  (CallFunction|GrosKKKIPU)
  (Actor|DestroyActor (Variables|Default|GetREF))
  (Rendering|SetVisibility (Variables|Default|GetDefaultSceneRoot) false true)
  (Audio|PlaySound2D "/Game/Matthys/Son/BreakFloor/DESTRUCTION_Wood_Debris_03_mono.DESTRUCTION_Wood_Debris_03_mono" 1.0 1.0 0.0 0 0)
  (Utilities|FlowControl|Delay 1e+01)
  (Actor|DestroyActor))

(event Custom|CanBreak
  (params (REF :type Actor%20Object%20Reference))
  (Variables|Default|SetREF REF)
  (Variables|/Script/Engine.PrimitiveComponent|SetbGenerateOverlapEvents (Variables|Default|GetBox) true)
  (Utilities|FlowControl|Delay 2.0)
  (Variables|/Script/Engine.PrimitiveComponent|SetbGenerateOverlapEvents (Variables|Default|GetBox) false))

(event Custom|GrosKKKIPU
  (bind _returnvalue (Game|GetPlayerController 0))
  (bind _as_bp_first_person_character (Variables|Default|GetAs%20BP%20First%20Person%20Character))
  (bind _as_bp_first_person_character_2 (Variables|Default|GetAs%20BP%20First%20Person%20Character))
  (bind _as_bp_first_person_character_3 (Variables|Default|GetAs%20BP%20First%20Person%20Character))
  (Utilities|IsValid (Variables|Default|GetCinematique)
    (:Is%20Valid
      (Variables|/Script/Engine.Pawn|SetbUseControllerRotationYaw _as_bp_first_person_character_3 false)
      (Variables|/Script/Engine.CameraComponent|SetbUsePawnControlRotation (Variables|/Game/Ugu/FirstPerson/Blueprints/BP_FirstPersonCharacter.BP_FirstPersonCharacter_C|GetFirstPersonCamera _as_bp_first_person_character_3) false)
      (if (Variables|Default|GetbEntrePont?)
        (Input|DisableInput (Game|GetPlayerCharacter 0) _returnvalue)
        (Game|Player|SetViewTargetwithBlend _returnvalue (Variables|Default|Getcamera_Ref) 1.0 "VTBlend_Linear" 3.0 false)
        (bind _returnvalue_2 (Sequencer|Player|CreateLevelSequencePlayer (Variables|Default|GetCinematique)))
        (Sequencer|Player|Play _returnvalue_2 :!class /Script/MovieScene.MovieSceneSequencePlayer)
        (Utilities|FlowControl|Delay 5.0)
        (Transformation|SetWorldLocation (Variables|/Script/Engine.Actor|GetRootComponent (Game|GetPlayerCharacter 0)) (Transformation|GetActorLocation (Variables|Default|GetRef_Player_Location)) false false)
        (Pawn|SetControlRotation (Game|GetPlayerController 0) (Math|Rotator|FindLookatRotation (Transformation|GetActorLocation (Game|GetPlayerCharacter 0)) (Transformation|GetActorLocation (Variables|Default|GetTarget%20location%20camera))))
        (Variables|/Script/Engine.Pawn|SetbUseControllerRotationYaw _as_bp_first_person_character true)
        (Variables|/Script/Engine.CameraComponent|SetbUsePawnControlRotation (Variables|/Game/Ugu/FirstPerson/Blueprints/BP_FirstPersonCharacter.BP_FirstPersonCharacter_C|GetFirstPersonCamera _as_bp_first_person_character) true)
        (Game|Player|SetViewTargetwithBlend (Game|GetPlayerController 0) (Game|GetPlayerCharacter 0) 1.0 "VTBlend_Linear" 3.0 false)
        (Variables|/Game/Ugu/FirstPerson/Blueprints/BP_FirstPersonCharacter.BP_FirstPersonCharacter_C|SetbCanOpenDoorCale (Variables|Default|GetAs%20BP%20First%20Person%20Character) true)
        (Development|PrintString "Hello" true true "(R=1.000000,G=0.000000,B=0.079899,A=1.000000)")
        (bind _returnvalue_3 (UserInterface|CreateWidget "/Game/Ugu/BluePrint/UI/WBP_Prison.WBP_Prison_C"))
        (bind _output_get (Variables|Default|SetREF_UI _returnvalue_3))
        (UserInterface|Viewport|AddtoViewport _output_get 0)
        (Default|67 (Variables|Default|GetREF_QTE69))
        (Default|Input _output_get self)
        (else
          (Game|Player|SetViewTargetwithBlend (Game|GetPlayerController 0) (Variables|Default|Getcamera_Ref) 1.0 "VTBlend_Linear" 3.0 false)
          (bind _returnvalue_4 (Sequencer|Player|CreateLevelSequencePlayer (Variables|Default|GetCinematique)))
          (Sequencer|Player|Play _returnvalue_4 :!class /Script/MovieScene.MovieSceneSequencePlayer)
          (Utilities|FlowControl|Delay 3.1)
          (Transformation|SetWorldLocation (Variables|/Script/Engine.Actor|GetRootComponent (Game|GetPlayerCharacter 0)) (Transformation|GetActorLocation (Variables|Default|GetRef_Player_Location)) false false)
          (Pawn|SetControlRotation (Game|GetPlayerController 0) (Math|Rotator|FindLookatRotation (Transformation|GetActorLocation (Game|GetPlayerCharacter 0)) (Transformation|GetActorLocation (Variables|Default|GetTarget%20location%20camera))))
          (Variables|/Script/Engine.Pawn|SetbUseControllerRotationYaw _as_bp_first_person_character_2 true)
          (Variables|/Script/Engine.CameraComponent|SetbUsePawnControlRotation (Variables|/Game/Ugu/FirstPerson/Blueprints/BP_FirstPersonCharacter.BP_FirstPersonCharacter_C|GetFirstPersonCamera _as_bp_first_person_character_2) true)
          (Game|Player|SetViewTargetwithBlend (Game|GetPlayerController 0) (Game|GetPlayerCharacter 0) 1.0 "VTBlend_Linear" 3.0 false)
          (Development|PrintString "Verterbre")
          (Variables|/Game/Ugu/FirstPerson/Blueprints/BP_FirstPersonCharacter.BP_FirstPersonCharacter_C|SetbCanOpenDoorCale (Variables|Default|GetAs%20BP%20First%20Person%20Character) true)
          (Default|PlankFall (Variables|Default|GetREF_PlankFall)))))))

(event Custom|Remove_UI
  (bind _ref_ui (Variables|Default|GetREF_UI))
  (Development|PrintString (Utilities|GetDisplayName _ref_ui))
  (bind _foundwidgets (Widget|GetAllWidgetsOfClass "/Game/Ugu/BluePrint/UI/WBP_Prison.WBP_Prison_C" true))
  (for _array_element _foundwidgets
    (Widget|RemovefromParent _ref_ui))
  (bind _returnvalue (Sequencer|Player|CreateLevelSequencePlayer "/Game/Ugu/BluePrint/Cinematic/Cinematique_HINT2.Cinematique_HINT2"))
  (Sequencer|Player|Play _returnvalue :!class /Script/MovieScene.MovieSceneSequencePlayer)
  (Utilities|FlowControl|Delay 5.1)
  (Development|PrintString "FZadf")
  (bind _asbp_first_person_character (Utilities|Casting|CastToBP_FirstPersonCharacter (Game|GetPlayerCharacter 0))
    (:then
      (Default|JAAJ _asbp_first_person_character 3)
      (Game|Player|SetViewTargetwithBlend (Game|GetPlayerController 0) (Game|GetPlayerCharacter 0) 1.0 "VTBlend_Linear" 3.0 false)
      (Input|EnableInput (Game|GetPlayerCharacter 0) (Game|GetPlayerController 0)))
    (:CastFailed
      (Development|PrintString "POIURT"))))

(event EventBeginPlay
  (Variables|/Script/Engine.PrimitiveComponent|SetbGenerateOverlapEvents (Variables|Default|GetBox) false))

(fn ConstructionScript)