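; BP_Trap is an interactable trap that can teleport the player to a TeleportTarget and switch between closed and open visuals.
; Its Interact prompt starts hidden, turns toward the camera every tick, and is shown or hidden by the CanInteract and Can'tInteractObject events.
; Zaap stops player movement and moves them to the target, keeping their rotation.
; Open_Visibility separately swaps CloseTrap for OpenTrap.
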(event Custom|Zaap
  (bind _returnvalue (Game|GetPlayerCharacter 0))
  (bind _asbp_first_person_character (Utilities|Casting|CastToBP_FirstPersonCharacter _returnvalue))
  (Utilities|IsValid (Variables|Default|GetTeleportTarget)
    (:Is%20Valid
      (Components|Movement|StopMovementImmediately (Variables|/Script/Engine.Character|GetCharacterMovement _returnvalue))
      (Transformation|SetActorLocationAndRotation _returnvalue (Transformation|GetActorLocation (Variables|Default|GetTeleportTarget)) (Transformation|GetActorRotation _asbp_first_person_character)))))

(event Custom|Open_Visibility
  (Rendering|SetVisibility (Variables|Default|GetOpenTrap) true false)
  (Rendering|SetVisibility (Variables|Default|GetCloseTrap) false false))

(event EventTick
  (params (DeltaSeconds :type Float%20%28single-precision%29))
  (Transformation|SetWorldRotation (Variables|Default|GetInteract) (Math|Rotator|FindLookatRotation (Transformation|GetWorldLocation (Variables|Default|GetInteract)) (Camera|GetCameraLocation (Game|GetPlayerCameraManager 0))) false false))

(event EventCanInteract
  (Rendering|SetVisibility (Variables|Default|GetInteract) true false))

(event EventBeginPlay
  (Rendering|SetVisibility (Variables|Default|GetInteract) false false))

(event EventCan'tInteractObject
  (Rendering|SetVisibility (Variables|Default|GetInteract) false false))

(fn ConstructionScript)