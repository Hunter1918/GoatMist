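; BP_Trigger_UI is a trigger volume that shows a configurable UI widget while the first-person character stands inside its box.
; Begin overlap creates the widget class and adds it to the viewport if none exists, and end overlap removes and clears it.
; With After set, overlaps start disabled until the Tutoexplain event enables them.
; The Destroy_UI_Crouch event destroys the trigger actor.
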(event OnComponentBeginOverlap(Box)
  (params (OverlappedComponent :type Primitive%20Component%20Object%20Reference) (OtherActor :type Actor%20Object%20Reference) (OtherComp :type Primitive%20Component%20Object%20Reference) (OtherBodyIndex :type Integer) (bFromSweep :type Boolean) (SweepResult :type Hit%20Result%20Structure%20%28by%20ref%29))
  (Utilities|Casting|CastToBP_FirstPersonCharacter OtherActor)
  (Utilities|IsValid (Variables|Default|GetCurent_UI)
    (:Is%20Not%20Valid
      (bind _returnvalue (UserInterface|CreateWidget (Variables|Default|GetWidget%20Class)))
      (bind _output_get (Variables|Default|SetCurent_UI _returnvalue))
      (UserInterface|Viewport|AddtoViewport _output_get 0))))

(event OnComponentEndOverlap(Box)
  (params (OverlappedComponent :type Primitive%20Component%20Object%20Reference) (OtherActor :type Actor%20Object%20Reference) (OtherComp :type Primitive%20Component%20Object%20Reference) (OtherBodyIndex :type Integer))
  (Utilities|Casting|CastToBP_FirstPersonCharacter OtherActor)
  (Widget|RemovefromParent (Variables|Default|GetCurent_UI))
  (Variables|Default|SetCurent_UI 0))

(event Custom|Tuto%20explain
  (Variables|/Script/Engine.PrimitiveComponent|SetbGenerateOverlapEvents (Variables|Default|GetBox) true))

(event Custom|Destroy_UI_Crouch
  (Actor|DestroyActor))

(event EventBeginPlay
  (if (Variables|Default|GetAfter?)
    (Variables|/Script/Engine.PrimitiveComponent|SetbGenerateOverlapEvents (Variables|Default|GetBox) false)))

(fn ConstructionScript)