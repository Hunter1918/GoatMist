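; Staircase actor that opens hidden stairs through a cutscene, then shows the Cladigo UI.
; Open_Stairs disables blocking collision, swaps closed for open meshes, locks player input and aim, plays a sequence, then repositions the player and creates the widget.
; Each Sequence pin re-enters that shared open chain.
; RemoveUI hides the Cladigo pose, plays a hint cinematic, animates a dissolve on the character's material and restores camera, input and aim.
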(event Custom|RemoveUI
  (bind _cladigopose1 (Variables|Default|GetCladigoPose1))
  (Development|PrintString "JAJAJAJAJA")
  (Widget|RemovefromParent (Variables|Default|GetREF_UI))
  (Rendering|SetVisibility _cladigopose1 false false)
  (Collision|SetCollisionEnabled _cladigopose1 "NoCollision")
  (bind _returnvalue (Sequencer|Player|CreateLevelSequencePlayer "/Game/Ugu/BluePrint/Cinematic/Cinematique_HINT0.Cinematique_HINT0"))
  (Sequencer|Player|Play _returnvalue :!class /Script/MovieScene.MovieSceneSequencePlayer)
  (Utilities|FlowControl|Delay 2.0)
  (bind _asbp_first_person_character (Utilities|Casting|CastToBP_FirstPersonCharacter (Game|GetPlayerCharacter 0)))
  (bind _returnvalue_2 (Rendering|Material|CreateDynamicMaterialInstance (Variables|/Game/Ugu/FirstPerson/Blueprints/BP_FirstPersonCharacter.BP_FirstPersonCharacter_C|GetChara_Anim_Rig _asbp_first_person_character) 1 (Rendering|Material|GetMaterial (Variables|/Game/Ugu/FirstPerson/Blueprints/BP_FirstPersonCharacter.BP_FirstPersonCharacter_C|GetChara_Anim_Rig _asbp_first_person_character) 1) "None" :!class /Script/Engine.PrimitiveComponent))
  (bind _newtrack_0 (Timeline|Timeline PlayFromStart)
    (:Update
      (Rendering|Material|SetScalarParameterValue _returnvalue_2 "Disolve" _newtrack_0 :!class /Script/Engine.MaterialInstanceDynamic)
      (Utilities|FlowControl|Delay 3.2)
      (Game|Player|SetViewTargetwithBlend (Game|GetPlayerController 0) (Game|GetPlayerCharacter 0) 1.0 "VTBlend_Linear" 3.0 false)
      (Input|EnableInput (Game|GetPlayerCharacter 0) (Game|GetPlayerController 0))
      (Variables|/Game/Ugu/FirstPerson/Blueprints/BP_FirstPersonCharacter.BP_FirstPersonCharacter_C|SetbCanAIM (Variables|Default|GetAs%20BP%20First%20Person%20Character) true))))

(event Custom|Open_Stairs
  (bind _returnvalue (Game|GetPlayerController 0))
  (bind _returnvalue_2 (Game|GetPlayerController 0))
  (bind _returnvalue_3 (Game|GetPlayerCharacter 0))
  (bind _returnvalue_4 (Game|GetPlayerCharacter 0))
  (bind _returnvalue_5 (Game|GetPlayerCharacter 0))
  (Utilities|FlowControl|Sequence
    (:then_0
      (Collision|SetCollisionEnabled (Variables|Default|GetStaticMesh12) "NoCollision"))
    (:then_1
      (Collision|SetCollisionEnabled (Variables|Default|GetStaticMesh13) "NoCollision"))
    (:then_2
      (Collision|SetCollisionEnabled (Variables|Default|GetStaticMesh17) "NoCollision"))
    (:then_3
      (Collision|SetCollisionEnabled (Variables|Default|GetStaticMesh14) "NoCollision"))
    (:then_4
      (Collision|SetCollisionEnabled (Variables|Default|GetStaticMesh15) "NoCollision"))
    (:then_5
      (Collision|SetCollisionEnabled (Variables|Default|GetStaticMesh16) "NoCollision"))
    (:then_6
      (Collision|SetCollisionEnabled (Variables|Default|GetStairsClose) "NoCollision")))
  (Rendering|SetVisibility (Variables|Default|GetStairsOpen) true true)
  (Rendering|SetVisibility (Variables|Default|GetStairsClose) false true)
  (Rendering|SetVisibility (Variables|Default|GetCladigoPose1) true false)
  (Collision|SetCollisionEnabled (Variables|Default|GetStairsOpen) "QueryAndPhysics")
  (bind _asbp_first_person_character (Utilities|Casting|CastToBP_FirstPersonCharacter _returnvalue_4))
  (bind _output_get (Variables|Default|SetAs%20BP%20First%20Person%20Character _asbp_first_person_character))
  (Variables|/Script/Engine.Pawn|SetbUseControllerRotationYaw _output_get false)
  (Variables|/Script/Engine.CameraComponent|SetbUsePawnControlRotation (Variables|/Game/Ugu/FirstPerson/Blueprints/BP_FirstPersonCharacter.BP_FirstPersonCharacter_C|GetFirstPersonCamera (Variables|Default|GetAs%20BP%20First%20Person%20Character)) false)
  (Variables|/Game/Ugu/FirstPerson/Blueprints/BP_FirstPersonCharacter.BP_FirstPersonCharacter_C|SetbCanAIM _output_get false)
  (Default|RecallKnife _output_get)
  (Input|DisableInput _returnvalue_4 _returnvalue_2)
  (Game|Player|SetViewTargetwithBlend _returnvalue_2 (Variables|Default|GetREF%20Camera%201) 1.0 "VTBlend_Linear" 3.0 false)
  (bind _returnvalue_6 (Sequencer|Player|CreateLevelSequencePlayer (Variables|Default|GetCinematic1)))
  (Sequencer|Player|Play _returnvalue_6 :!class /Script/MovieScene.MovieSceneSequencePlayer)
  (Utilities|FlowControl|Delay 5.6)
  (Transformation|SetWorldLocation (Variables|/Script/Engine.Actor|GetRootComponent _returnvalue_5) (Transformation|GetActorLocation (Variables|Default|GetTarget%20location%20Player)) false false)
  (Transformation|SetWorldRotation (Variables|/Script/Engine.Actor|GetRootComponent _returnvalue_3) "0.000000,-180.000000,0.000000" false false)
  (Pawn|SetControlRotation _returnvalue (Math|Rotator|FindLookatRotation (Transformation|GetActorLocation _returnvalue_5) (Transformation|GetActorLocation (Variables|Default|GetTarget%20location%20camera))))
  (Utilities|FlowControl|Delay 0.2)
  (Variables|/Script/Engine.Pawn|SetbUseControllerRotationYaw (Variables|Default|GetAs%20BP%20First%20Person%20Character) true)
  (Variables|/Script/Engine.CameraComponent|SetbUsePawnControlRotation (Variables|/Game/Ugu/FirstPerson/Blueprints/BP_FirstPersonCharacter.BP_FirstPersonCharacter_C|GetFirstPersonCamera (Variables|Default|GetAs%20BP%20First%20Person%20Character)) true)
  (Game|Player|SetViewTargetwithBlend _returnvalue _returnvalue_3 0.0 "VTBlend_Linear" 3.0 false)
  (Variables|/Game/Ugu/FirstPerson/Blueprints/BP_FirstPersonCharacter.BP_FirstPersonCharacter_C|SetbCanAIM (Variables|Default|GetAs%20BP%20First%20Person%20Character) true)
  (bind _returnvalue_7 (UserInterface|CreateWidget "/Game/Ugu/BluePrint/UI/WBP_Cladigo.WBP_Cladigo_C"))
  (bind _output_get_2 (Variables|Default|SetREF_UI _returnvalue_7))
  (UserInterface|Viewport|AddtoViewport _returnvalue_7 0)
  (Utilities|FlowControl|Delay 2.0)
  (Default|Input _returnvalue_7 self))

(event EventBeginPlay
  (Rendering|SetVisibility (Variables|Default|GetStairsOpen) false true)
  (Collision|SetCollisionEnabled (Variables|Default|GetStairsOpen) "NoCollision"))

(fn ConstructionScript)