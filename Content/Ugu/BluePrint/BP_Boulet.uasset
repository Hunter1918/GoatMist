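; BP_Boulet is an interactable cannonball source that hands out cannonballs on demand.
; GetBoulet spawns a BP_Boulet_De_Canon at its location, stores the reference and calls BouletEnMain on it, leaving the source in place.
; Its Interact prompt starts hidden, is toggled by CanInteract and Can'tInteractObject, and turns every tick to face the player camera.
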(event Custom|GetBoulet
  (bind _returnvalue (Game|SpawnActorfromClass "/Game/Ugu/BluePrint/BP_Boulet_De_Canon.BP_Boulet_De_Canon_C" (Math|Transform|MakeTransform (Transformation|GetActorLocation) "0, 0, 0" "1.000000,1.000000,1.000000") "Undefined" "MultiplyWithRoot" 0 0))
  (bind _output_get (Variables|Default|SetRef_BP_Boulet _returnvalue))
  (Default|BouletEnMain _output_get))

(event EventTick
  (params (DeltaSeconds :type Float%20%28single-precision%29))
  (Transformation|SetWorldRotation (Variables|Default|GetInteract) (Math|Rotator|FindLookatRotation (Transformation|GetWorldLocation (Variables|Default|GetInteract)) (Camera|GetCameraLocation (Game|GetPlayerCameraManager 0))) false false))

(event EventCanInteract
  (Rendering|SetVisibility (Variables|Default|GetInteract) true false))

(event EventBeginPlay
  (Rendering|SetVisibility (Variables|Default|GetInteract) false false))

(event EventCan'tInteractObject
  (Rendering|SetVisibility (Variables|Default|GetInteract) false false))

(fn ConstructionScript)