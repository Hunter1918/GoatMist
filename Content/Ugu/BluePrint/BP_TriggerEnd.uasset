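; BP_TriggerEnd is a trigger box that starts the ending sequence when the first-person character enters it.
; It switches off its overlap events so it fires once, then plays the Cinematic level sequence.
; After a Duration delay it starts a camera fade and shows the WBP_EndImage widget with its fade animation.
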(event OnComponentBeginOverlap(Box)
  (params (OverlappedComponent :type Primitive%20Component%20Object%20Reference) (OtherActor :type Actor%20Object%20Reference) (OtherComp :type Primitive%20Component%20Object%20Reference) (OtherBodyIndex :type Integer) (bFromSweep :type Boolean) (SweepResult :type Hit%20Result%20Structure%20%28by%20ref%29))
  (Utilities|Casting|CastToBP_FirstPersonCharacter OtherActor)
  (Variables|/Script/Engine.PrimitiveComponent|SetbGenerateOverlapEvents (Variables|Default|GetBox) false)
  (bind _returnvalue (Sequencer|Player|CreateLevelSequencePlayer (Variables|Default|GetCinematic)))
  (Sequencer|Player|Play _returnvalue :!class /Script/MovieScene.MovieSceneSequencePlayer)
  (Utilities|FlowControl|Delay (Variables|Default|GetDuration))
  (CameraFades|StartCameraFade :self (Game|GetPlayerCameraManager 0) :ToAlpha 1.0 :Duration 2.0)
  (bind _returnvalue_2 (UserInterface|CreateWidget "/Game/Ugu/BluePrint/UI/WBP_EndImage.WBP_EndImage_C"))
  (UserInterface|Viewport|AddtoViewport _returnvalue_2 0)
  (Default|FadeAnim _returnvalue_2))

(fn ConstructionScript)