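; BP_CutRope is a rope that a BP_RopeKnife can cut to trigger a mechanism in the level.
; When the knife overlaps its Box, boolean flags named 1, 2 and 3 select which referenced actor reacts: stairs open, an étagère drops or a plank drops.
; Each branch also detaches the adjoining ends of the two cable components and turns off the Box's overlap events.
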(event OnComponentBeginOverlap(Box)
  (params (OverlappedComponent :type Primitive%20Component%20Object%20Reference) (OtherActor :type Actor%20Object%20Reference) (OtherComp :type Primitive%20Component%20Object%20Reference) (OtherBodyIndex :type Integer) (bFromSweep :type Boolean) (SweepResult :type Hit%20Result%20Structure%20%28by%20ref%29))
  (Utilities|Casting|CastToBP_RopeKnife OtherActor)
  (Utilities|FlowControl|Sequence
    (:then_0
      (if (Variables|Default|Get1)
        (Variables|/Script/CableComponent.CableComponent|SetbAttachEnd (Variables|Default|GetCable1) false)
        (Variables|/Script/CableComponent.CableComponent|SetbAttachStart (Variables|Default|GetCable) false)
        (Variables|/Script/Engine.PrimitiveComponent|SetbGenerateOverlapEvents (Variables|Default|GetBox) false)
        (Default|OpenStairs (Variables|Default|GetRef_Stairs))))
    (:then_1
      (if (Variables|Default|Get2)
        (Variables|/Script/CableComponent.CableComponent|SetbAttachEnd (Variables|Default|GetCable1) false)
        (Variables|/Script/CableComponent.CableComponent|SetbAttachStart (Variables|Default|GetCable) false)
        (Variables|/Script/Engine.PrimitiveComponent|SetbGenerateOverlapEvents (Variables|Default|GetBox) false)
        (Default|Drop (Variables|Default|GetREF_Etagere))))
    (:then_2
      (if (Variables|Default|Get3)
        (Variables|/Script/CableComponent.CableComponent|SetbAttachEnd (Variables|Default|GetCable1) false)
        (Variables|/Script/CableComponent.CableComponent|SetbAttachStart (Variables|Default|GetCable) false)
        (Variables|/Script/Engine.PrimitiveComponent|SetbGenerateOverlapEvents (Variables|Default|GetBox) false)
        (Default|DropPlank (Variables|Default|GetREF_Plank))))))

(fn ConstructionScript)