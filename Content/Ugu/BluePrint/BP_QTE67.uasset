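; BP_QTE67 is a crab QTE trigger actor that starts hidden with box collision off until its "67" event reveals it and enables the box.
; When the first-person character overlaps the box, it disables overlaps and starts its QTEID through the QTE manager reference.
; A reset event re-arms the trigger.
; A destroy event drives a dissolve parameter on a dynamic crab material via timeline, then destroys the actor after a delay.
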(event OnComponentBeginOverlap(Box)
  (params (OverlappedComponent :type Primitive%20Component%20Object%20Reference) (OtherActor :type Actor%20Object%20Reference) (OtherComp :type Primitive%20Component%20Object%20Reference) (OtherBodyIndex :type Integer) (bFromSweep :type Boolean) (SweepResult :type Hit%20Result%20Structure%20%28by%20ref%29))
  (bind _qtemanager_ref (Variables|Default|GetQTEManager%20Ref))
  (Utilities|Casting|CastToBP_FirstPersonCharacter OtherActor)
  (Variables|/Script/Engine.PrimitiveComponent|SetbGenerateOverlapEvents (Variables|Default|GetBox) false)
  (Utilities|IsValid _qtemanager_ref
    (:Is%20Valid
      (Default|StartQTE _qtemanager_ref (Variables|Default|GetQTE_ID) self))))

(event Custom|ResetQTETrigger
  (Variables|/Script/Engine.PrimitiveComponent|SetbGenerateOverlapEvents (Variables|Default|GetBox) true))

(event Custom|Destroy_Actor
  (bind _crabe1 (Variables|Default|GetCrabe1))
  (Variables|/Script/Engine.PrimitiveComponent|SetbGenerateOverlapEvents (Variables|Default|GetBox) false)
  (bind _returnvalue (Rendering|Material|CreateDynamicMaterialInstance _crabe1 0 (Rendering|Material|GetMaterial _crabe1 0) "None" :!class /Script/Engine.PrimitiveComponent))
  (bind _newtrack_0 (Timeline|Timeline PlayFromStart)
    (:Update
      (Rendering|Material|SetScalarParameterValue _returnvalue "Disolve" _newtrack_0 :!class /Script/Engine.MaterialInstanceDynamic)
      (Utilities|FlowControl|Delay 3.0)
      (Actor|DestroyActor))))

(event Custom|67
  (Collision|SetCollisionEnabled (Variables|Default|GetBox) "QueryAndPhysics")
  (Rendering|SetVisibility (Variables|Default|GetCrabe1) true true))

(event EventBeginPlay
  (Collision|SetCollisionEnabled (Variables|Default|GetBox) "NoCollision")
  (Rendering|SetVisibility (Variables|Default|GetCrabe1) false true))

(fn ConstructionScript)