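; BP_Door_Cale is a one-way door that swings open once, with an interaction prompt gated by the player character's CanOpenDoorCale flag.
; CanInteract shows the Interact component only when that flag is set, and Can'tInteractObject hides it.
; Open_Door_Cale does not check the flag; it sets DoorOpen and runs a Timeline that yaws the mesh 90 degrees.
; Tick turns the prompt toward the camera and destroys it once opened.
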(event Custom|Open_Door_Cale
  (if (not (Variables|Default|GetDoor%20Open))
    (Variables|Default|SetDoor%20Open true)
    (bind _door_track (Timeline|Timeline PlayFromStart)
      (:Update
        (Transformation|SetRelativeRotation (Variables|Default|GetpolySurface275) (Math|Rotator|MakeRotator 0.0 0.0 (Math|Float|Lerp 0.0 9e+01 _door_track)) false false)))))

(event EventTick
  (params (DeltaSeconds :type Float%20%28single-precision%29))
  (if (Variables|Default|GetbIsValid)
    (Transformation|SetWorldRotation (Variables|Default|GetInteract) (Math|Rotator|FindLookatRotation (Transformation|GetWorldLocation (Variables|Default|GetInteract)) (Camera|GetCameraLocation (Game|GetPlayerCameraManager 0))) false false)
    (if (Variables|Default|GetDoor%20Open)
      (Components|DestroyComponent (Variables|Default|GetInteract))
      (Variables|Default|SetbIsValid false))))

(event EventCanInteract
  (bind _asbp_first_person_character (Utilities|Casting|CastToBP_FirstPersonCharacter (Game|GetPlayerCharacter 0)))
  (if (Variables|/Game/Ugu/FirstPerson/Blueprints/BP_FirstPersonCharacter.BP_FirstPersonCharacter_C|GetbCanOpenDoorCale _asbp_first_person_character)
    (Rendering|SetVisibility (Variables|Default|GetInteract) true false)))

(event EventBeginPlay
  (Rendering|SetVisibility (Variables|Default|GetInteract) false false))

(event EventCan'tInteractObject
  (Rendering|SetVisibility (Variables|Default|GetInteract) false false))

(fn ConstructionScript)