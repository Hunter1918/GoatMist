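; One-shot trigger that plays a book-reading cinematic when the first-person character overlaps its box.
; On overlap it disables input, blends to a cinematic camera, plays a sequence, then shows WBP_BookRead and passes itself to the widget.
; The FTG event removes the widget, plays a hint sequence, sets the character rig's Disolve material parameter, then restores the player view and input.
; Fixed delays time each step.
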(event OnComponentBeginOverlap(Box)
  (params (OverlappedComponent :type Primitive%20Component%20Object%20Reference) (OtherActor :type Actor%20Object%20Reference) (OtherComp :type Primitive%20Component%20Object%20Reference) (OtherBodyIndex :type Integer) (bFromSweep :type Boolean) (SweepResult :type Hit%20Result%20Structure%20%28by%20ref%29))
  (Utilities|Casting|CastToBP_FirstPersonCharacter OtherActor)
  (Input|DisableInput (Game|GetPlayerCharacter 0) (Game|GetPlayerController 0))
  (Variables|/Script/Engine.PrimitiveComponent|SetbGenerateOverlapEvents (Variables|Default|GetBox) false)
  (Game|Player|SetViewTargetwithBlend (Game|GetPlayerController 0) (Variables|Default|GetREF%20Camera%201) 1.0 "VTBlend_Linear" 3.0 false)
  (bind _returnvalue (Sequencer|Player|CreateLevelSequencePlayer (Variables|Default|GetCinematic1)))
  (Sequencer|Player|Play _returnvalue :!class /Script/MovieScene.MovieSceneSequencePlayer)
  (Utilities|FlowControl|Delay 4.0)
  (bind _returnvalue_2 (UserInterface|CreateWidget "/Game/Ugu/BluePrint/UI/WBP_BookRead.WBP_BookRead_C"))
  (bind _output_get (Variables|Default|SetREF_UI _returnvalue_2))
  (UserInterface|Viewport|AddtoViewport _returnvalue_2 0)
  (Utilities|FlowControl|Delay 2.0)
  (Default|Input _returnvalue_2 self))

(event Custom|FTG
  (Development|PrintString "JAJAJAJAJA")
  (Widget|RemovefromParent (Variables|Default|GetREF_UI))
  (bind _returnvalue (Sequencer|Player|CreateLevelSequencePlayer "/Game/Ugu/BluePrint/Cinematic/Cinematique_HINT1.Cinematique_HINT1"))
  (Sequencer|Player|Play _returnvalue :!class /Script/MovieScene.MovieSceneSequencePlayer)
  (Utilities|FlowControl|Delay 2.0)
  (bind _asbp_first_person_character (Utilities|Casting|CastToBP_FirstPersonCharacter (Game|GetPlayerCharacter 0)))
  (bind _returnvalue_2 (Rendering|Material|CreateDynamicMaterialInstance (Variables|/Game/Ugu/FirstPerson/Blueprints/BP_FirstPersonCharacter.BP_FirstPersonCharacter_C|GetChara_Anim_Rig _asbp_first_person_character) 0 (Rendering|Material|GetMaterial (Variables|/Game/Ugu/FirstPerson/Blueprints/BP_FirstPersonCharacter.BP_FirstPersonCharacter_C|GetChara_Anim_Rig _asbp_first_person_character) 0) "None" :!class /Script/Engine.PrimitiveComponent))
  (Rendering|Material|SetScalarParameterValue _returnvalue_2 "Disolve" 2e+02 :!class /Script/Engine.MaterialInstanceDynamic)
  (Utilities|FlowControl|Delay 3.2)
  (Game|Player|SetViewTargetwithBlend (Game|GetPlayerController 0) (Game|GetPlayerCharacter 0) 1.0 "VTBlend_Linear" 3.0 false)
  (Input|EnableInput (Game|GetPlayerCharacter 0) (Game|GetPlayerController 0)))

(fn ConstructionScript)