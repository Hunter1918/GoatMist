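; BP_SignLockRED3 is a rotating puzzle lock piece that reports to the first-person character whether it sits in the correct position.
; ActiveFace turns the Pivot a quarter turn by timeline, holding the player's CylinderIsActivate flag off until shortly after it finishes.
; Box overlap with the Correct component sets IsValid, which the timeline's Update checks and clears, sending a delayed EventPuzzle4 true or false to the character.
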(event OnComponentBeginOverlap(Box)
  (params (OverlappedComponent :type Primitive%20Component%20Object%20Reference) (OtherActor :type Actor%20Object%20Reference) (OtherComp :type Primitive%20Component%20Object%20Reference) (OtherBodyIndex :type Integer) (bFromSweep :type Boolean) (SweepResult :type Hit%20Result%20Structure%20%28by%20ref%29))
  (if (== OtherComp (Variables|Default|GetCorrect))
    (Variables|Default|SetbIsValid true)))

(event OnComponentEndOverlap(Box)
  (params (OverlappedComponent :type Primitive%20Component%20Object%20Reference) (OtherActor :type Actor%20Object%20Reference) (OtherComp :type Primitive%20Component%20Object%20Reference) (OtherBodyIndex :type Integer))
  (if (== OtherComp (Variables|Default|GetCorrect))
    (Variables|Default|SetbIsValid false)))

(event Custom|ActiveFace
  (bind _returnvalue (Game|Player|GetPlayerPawn 0))
  (bind _asbp_first_person_character (Utilities|Casting|CastToBP_FirstPersonCharacter (Game|Player|GetPlayerPawn 0)))
  (Variables|/Game/Ugu/FirstPerson/Blueprints/BP_FirstPersonCharacter.BP_FirstPersonCharacter_C|SetbCylinderIsActivate _asbp_first_person_character false)
  (Variables|Default|SetStartRotation (Variables|Default|GetCurrentRotation))
  (Variables|Default|SetTargetRotation (+ (Variables|Default|GetCurrentRotation) 9e+01))
  (bind _newtrack_0 (Timeline|Timeline PlayFromStart)
    (:Update
      (Variables|Default|SetNew%20Track%200 _newtrack_0)
      (Transformation|SetRelativeRotation (Variables|Default|GetPivot) (Math|Rotator|MakeRotator 0.0 0.0 (Math|Float|Lerp (Variables|Default|GetStartRotation) (Variables|Default|GetTargetRotation) _newtrack_0)) false false)
      (bind _asbp_first_person_character_2 (Utilities|Casting|CastToBP_FirstPersonCharacter _returnvalue))
      (if (Variables|Default|GetbIsValid)
        (Variables|Default|SetbIsValid false)
        (Utilities|FlowControl|Delay 1.0)
        (Development|PrintString "YIpiiii")
        (Default|EventPuzzle4 _asbp_first_person_character_2 true)
        (else
          (Utilities|FlowControl|Delay 1.0)
          (Development|PrintString "T'es trompé")
          (Default|EventPuzzle4 _asbp_first_person_character_2 false))))
    (:Finished
      (Variables|Default|SetCurrentRotation (Variables|Default|GetTargetRotation))
      (bind _asbp_first_person_character_3 (Utilities|Casting|CastToBP_FirstPersonCharacter _returnvalue))
      (Utilities|FlowControl|Delay 0.5)
      (Variables|/Game/Ugu/FirstPerson/Blueprints/BP_FirstPersonCharacter.BP_FirstPersonCharacter_C|SetbCylinderIsActivate _asbp_first_person_character_3 true))))

(fn ConstructionScript)