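; Puzzle-room prop actor, apparently for a cut-rope setup, whose Drop event releases three crates and a bottle and tilts their rig.
; Drop enables physics on the props, then separate timelines drive a "Disolve" parameter on each one's dynamic material instances.
; A Delay chained to each timeline's Update destroys the prop about three seconds after its dissolve starts.
; In parallel, another timeline pitches the Pivot component to 40 degrees.
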(event Custom|Drop
  (bind _prop_crate (Variables|Default|GetPROP_Crate))
  (bind _prop_crate2 (Variables|Default|GetPROP_Crate2))
  (bind _prop_crate1 (Variables|Default|GetPROP_Crate1))
  (bind _prop_bottle_l (Variables|Default|GetPROP_Bottle_L))
  (Utilities|FlowControl|Sequence
    (:then_0
      (Physics|SetSimulatePhysics _prop_crate true)
      (Utilities|FlowControl|Sequence
        (:then_0
          (bind _returnvalue (Rendering|Material|CreateDynamicMaterialInstance _prop_crate 0 (Rendering|Material|GetMaterial _prop_crate 0) "None" :!class /Script/Engine.PrimitiveComponent))
          (bind _returnvalue_2 (Rendering|Material|CreateDynamicMaterialInstance _prop_crate 1 (Rendering|Material|GetMaterial _prop_crate 1) "None" :!class /Script/Engine.PrimitiveComponent))
          (bind _newtrack_0 (Timeline|Timeline PlayFromStart)
            (:Update
              (Rendering|Material|SetScalarParameterValue _returnvalue "Disolve" _newtrack_0 :!class /Script/Engine.MaterialInstanceDynamic)
              (Rendering|Material|SetScalarParameterValue _returnvalue_2 "Disolve" _newtrack_0 :!class /Script/Engine.MaterialInstanceDynamic)
              (Utilities|FlowControl|Delay 3.0)
              (Variables|/Script/Engine.PrimitiveComponent|SetbGenerateOverlapEvents _prop_crate false)
              (Components|DestroyComponent _prop_crate))))
        (:then_1
          (bind _returnvalue_3 (Rendering|Material|CreateDynamicMaterialInstance _prop_crate1 0 (Rendering|Material|GetMaterial _prop_crate1 0) "None" :!class /Script/Engine.PrimitiveComponent))
          (bind _returnvalue_4 (Rendering|Material|CreateDynamicMaterialInstance _prop_crate1 1 (Rendering|Material|GetMaterial _prop_crate1 1) "None" :!class /Script/Engine.PrimitiveComponent))
          (bind _newtrack_0_2 (Timeline|Timeline_0 PlayFromStart)
            (:Update
              (Rendering|Material|SetScalarParameterValue _returnvalue_3 "Disolve" _newtrack_0_2 :!class /Script/Engine.MaterialInstanceDynamic)
              (Rendering|Material|SetScalarParameterValue _returnvalue_4 "Disolve" _newtrack_0_2 :!class /Script/Engine.MaterialInstanceDynamic)
              (Utilities|FlowControl|Delay 3.0)
              (Variables|/Script/Engine.PrimitiveComponent|SetbGenerateOverlapEvents _prop_crate1 false)
              (Components|DestroyComponent _prop_crate1))))
        (:then_2
          (bind _returnvalue_5 (Rendering|Material|CreateDynamicMaterialInstance _prop_crate2 0 (Rendering|Material|GetMaterial _prop_crate2 0) "None" :!class /Script/Engine.PrimitiveComponent))
          (bind _returnvalue_6 (Rendering|Material|CreateDynamicMaterialInstance _prop_crate2 1 (Rendering|Material|GetMaterial _prop_crate2 1) "None" :!class /Script/Engine.PrimitiveComponent))
          (bind _newtrack_0_3 (Timeline|Timeline_1 PlayFromStart)
            (:Update
              (Rendering|Material|SetScalarParameterValue _returnvalue_5 "Disolve" _newtrack_0_3 :!class /Script/Engine.MaterialInstanceDynamic)
              (Rendering|Material|SetScalarParameterValue _returnvalue_6 "Disolve" _newtrack_0_3 :!class /Script/Engine.MaterialInstanceDynamic)
              (Utilities|FlowControl|Delay 3.0)
              (Variables|/Script/Engine.PrimitiveComponent|SetbGenerateOverlapEvents _prop_crate2 false)
              (Components|DestroyComponent _prop_crate2))))
        (:then_3
          (bind _returnvalue_7 (Rendering|Material|CreateDynamicMaterialInstance _prop_bottle_l 0 (Rendering|Material|GetMaterial _prop_bottle_l 0) "None" :!class /Script/Engine.PrimitiveComponent))
          (bind _newtrack_0_4 (Timeline|Timeline_2 PlayFromStart)
            (:Update
              (Rendering|Material|SetScalarParameterValue _returnvalue_7 "Disolve" _newtrack_0_4 :!class /Script/Engine.MaterialInstanceDynamic)
              (Utilities|FlowControl|Delay 3.0)
              (Variables|/Script/Engine.PrimitiveComponent|SetbGenerateOverlapEvents _prop_bottle_l false)
              (Components|DestroyComponent _prop_bottle_l))))))
    (:then_1
      (bind _newtrack_0_5 (Timeline|Timeline_3 Play)
        (:Update
          (Transformation|SetRelativeRotation (Variables|Default|GetPivot) (Math|Rotator|MakeRotator 0.0 (Math|Float|Lerp 0.0 4e+01 _newtrack_0_5) 0.0) false false))))))

(fn ConstructionScript)